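; TrapBP is a landmine that arms itself a few seconds after spawning and explodes when a living zombie steps on it.
; Once armed, Tick runs a small Pawn sphere trace with debug drawing and casts the hit to AIZombie to check its health.
; A valid hit plays explosion effects and attenuated sound, applies radial damage, then destroys the actor after a short delay.
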(event EventBeginPlay
  ;[1 1 1] Arming the bomb
  (Utilities|FlowControl|Delay 5.0)
  (Variables|Default|SetIsArmed true))

(event EventTick
  (params (DeltaSeconds :type Float%20%28single-precision%29))
  (bind _returnvalue (Transformation|GetActorLocation))
  ;[1 1 1] Check if someone walks oni t
  (if (Variables|Default|GetIsArmed)
    (bind (_outhit _returnvalue_2) (Collision|SphereTraceForObjects _returnvalue (+ _returnvalue "0.000000,0.000000,15.000000") 5e+01 (Utilities|Array|MakeArray "ObjectTypeQuery3") false 0 "ForDuration"))
    ;[1 1 1] Make sure triggering zombie isn't dead
    (if _returnvalue_2
      (bind _asaizombie_c (Utilities|Casting|CastToAIZombie (.HitActor (Collision|BreakHitResult _outhit))))
      (if (> (Variables|/Game/Character/Zombie/AIZombie.AIZombie_C|GetHealth _asaizombie_c) 0.0)
        (Variables|Default|SetisExploding true)
        ;[1 1 1] Effects and sound
        (if (Variables|Default|GetisExploding)
          (Effects|SpawnEmitteratLocation "/Game/Particles/Explosion.Explosion" _returnvalue)
          (Audio|PlaySoundatLocation "/Game/Sounds/LandmineBoom.LandmineBoom" _returnvalue 0.7 1.0 0.0 "/Game/Sounds/GunshotAttenuate.GunshotAttenuate")
          ;[1 1 1] KILL EVERYTHING
          (Game|Damage|ApplyRadialDamage 4e+02 _returnvalue 4e+02 0 0 0 0 false "ECC_Visibility")
          (Utilities|FlowControl|Delay 0.5)
          (Actor|DestroyActor))))))

(fn ConstructionScript)