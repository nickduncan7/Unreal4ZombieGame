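; SurvivalTestHUD is a HUD Blueprint that draws a crosshair texture near the middle of the screen.
; On each DrawHUD event it converts the screen width and height to floats and passes them through math expressions, which appear to halve each and subtract a fixed pixel offset.
; The results position a scaled-down DrawTextureSimple call, and the construction script is empty.
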(event EventDrawHUD
  (params (SizeX :type Integer) (SizeY :type Integer))
  (Class|HUD|DrawTextureSimple "/Game/Textures/Mine/Crosshair.Crosshair" (|(x/2)-20 (Math|Conversions|ToFloat(Integer) SizeX)) (|(y/2)-20 (Math|Conversions|ToFloat(Integer) SizeY)) 0.1 false))

(fn ConstructionScript)