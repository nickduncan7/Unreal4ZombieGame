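; LightMeshBP is a prop actor that aligns itself with a referenced LightActor, presumably as the visible mesh for that light.
; On BeginPlay it copies the light actor's rotation and location once and sets OriginalRotation to zero.
; Tick holds only an empty branch, and unconnected nodes hint at an unfinished or disabled rotation of LightMesh based on the player camera's position.
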(event `self.ReceiveBeginPlay`
  (bind _lightactor (`self.LightActor`))
  (`self.SetActorRotation` (`self.K2_GetActorRotation` _lightactor))
  (set `self.OriginalRotation` (struct))
  (`self.K2_SetActorLocation` (`self.K2_GetActorLocation` _lightactor)))

(event `self.ReceiveTick`
  (params (DeltaSeconds :type "Float (single-precision)"))
  (if true
    _))

(fn `UserConstructionScript`)